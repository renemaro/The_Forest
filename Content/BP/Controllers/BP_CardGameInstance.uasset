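; BP_CardGameInstance is the card game's game instance, holding a Storehouse map of item counts.
; AddItems merges an incoming item map into the Storehouse, summing values for existing keys and inserting new ones, then returns true.
; GetItems returns the whole Storehouse map.
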(fn AddItems
  (params (ItemsList :type Map%20of%20Names%20to%20Integers))
  (bind _keys (Utilities|Map|Keys ItemsList))
  (for _array_element _keys
    (if (.ReturnValue (Utilities|Map|Find (Variables|Default|GetStorehouse) _array_element))
      (Utilities|Map|Add (Variables|Default|GetStorehouse) _array_element (+ (.Value (Utilities|Map|Find (Variables|Default|GetStorehouse) _array_element)) (.Value (Utilities|Map|Find ItemsList _array_element))))
      (else
        (Utilities|Map|Add (Variables|Default|GetStorehouse) _array_element (.Value (Utilities|Map|Find ItemsList _array_element))))))
  (return true))

(fn GetItems
  (return (Variables|Default|GetStorehouse)))