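; Game mode Blueprint for a card game that holds the current skills, abilities and deck data.
; On BeginPlay it sets scalability quality to Epic.
; A SetSkill event stores the incoming skills, and getter functions return the skills, abilities and deck data.
; The abilities and deck data are only read in this graph, with no setters here.
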(event EventBeginPlay
  (Class|AutomationBlueprintFunctionLibrary|SetScalabilityQualitytoEpic))

(event EventSetSkill
  (params (Skills :type Map%20of%20Names%20to%20Integers))
  (Variables|Default|SetCurrentSkils Skills))

(fn ConstructionScript)

(fn GetAbilities
  (return (Variables|Default|GetCurrentAbilities)))

(fn GetDeckData
  (return (Variables|Default|GetDeck%20Data)))

(fn GetSkills
  (return (Variables|Default|GetCurrentSkils)))