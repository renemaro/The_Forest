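; Player controller for a card game that builds the level deck and lays it out as three rows of BP_CardPar cards.
; On BeginPlay it expands the GameMode's deck data into a card list, shuffles it, spawns the rows and reveals three cards in each.
; TryToUseCard calls MoveCardRow, which removes the card from its row, messages the rest to move, activates one and refreshes visibility.
; SpawnCardsOLD is an uncalled earlier spawner.
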(event EventBeginPlay
  (bind _deckdata (Class|INTCardGameMode|GetDeckData(Message) (Game|GetGameMode)))
  (CallFunction|CreateLevelDeck _deckdata)
  (Utilities|Array|Shuffle (Variables|Default|GetLevelDeck))
  (CallFunction|SpawnCardsfromMainDeck)
  (CallFunction|StartingCardsSetting))

(fn ConstructionScript)

(fn SpawnCardsOLD
  (for _index (range 0 2)
    (bind _output_get (Variables|Default|SetZoffset (+ (Variables|Default|GetZoffset) 3e+01)))
    (bind _output_get_2 (Variables|Default|SetStartingPosition (+ (Variables|Default|GetStartingPosition) (Variables|Default|GetYoffset))))
    (bind _returnvalue (Game|SpawnActorfromClass "/Game/BP/Cards/BP_CardPar.BP_CardPar_C" (Math|Transform|MakeTransform (Math|Vector|MakeVector 0.0 _output_get_2 _output_get) "0, 0, 0" "1.000000,1.000000,1.000000") "Undefined" "MultiplyWithRoot" 0 (Utilities|Array|Get(acopy) (Variables|Default|GetLevelDeck)) 0))
    (Utilities|Array|RemoveIndex (Variables|Default|GetLevelDeck))
    (Utilities|Array|Add (Variables|Default|GetCurrentDeck) _returnvalue)
    (Utilities|FlowControl|DoOnce false
      (:Completed
        (Variables|/Game/BP/Cards/BP_CardPar.BP_CardPar_C|SetIsActive _returnvalue true))))
  (Variables|Default|SetZoffset -3e+01)
  (Variables|Default|SetStartingPosition 2e+02)
  (for _index_2 (range 0 2)
    (bind _output_get_3 (Variables|Default|SetZoffset (+ (Variables|Default|GetZoffset) 3e+01)))
    (bind _output_get_4 (Variables|Default|SetStartingPosition (+ (Variables|Default|GetStartingPosition) (Variables|Default|GetYoffset))))
    (bind _returnvalue_2 (Game|SpawnActorfromClass "/Game/BP/Cards/BP_CardPar.BP_CardPar_C" (Math|Transform|MakeTransform (Math|Vector|MakeVector 1.6e+02 _output_get_4 _output_get_3) "0, 0, 0" "1.000000,1.000000,1.000000") "Undefined" "MultiplyWithRoot" 0 (Utilities|Array|Get(acopy) (Variables|Default|GetLevelDeck)) 0))
    (Utilities|Array|RemoveIndex (Variables|Default|GetLevelDeck))
    (Utilities|Array|Add (Variables|Default|GetCurrentDeck) _returnvalue_2)
    (Utilities|FlowControl|DoOnce false
      (:Completed
        (Variables|/Game/BP/Cards/BP_CardPar.BP_CardPar_C|SetIsActive _returnvalue_2 true))))
  (Variables|Default|SetZoffset -3e+01)
  (Variables|Default|SetStartingPosition 2e+02)
  (for _index_3 (range 0 2)
    (bind _output_get_5 (Variables|Default|SetZoffset (+ (Variables|Default|GetZoffset) 3e+01)))
    (bind _output_get_6 (Variables|Default|SetStartingPosition (+ (Variables|Default|GetStartingPosition) (Variables|Default|GetYoffset))))
    (bind _returnvalue_3 (Game|SpawnActorfromClass "/Game/BP/Cards/BP_CardPar.BP_CardPar_C" (Math|Transform|MakeTransform (Math|Vector|MakeVector 3.2e+02 _output_get_6 _output_get_5) "0, 0, 0" "1.000000,1.000000,1.000000") "Undefined" "MultiplyWithRoot" 0 (Utilities|Array|Get(acopy) (Variables|Default|GetLevelDeck)) 0))
    (Utilities|Array|RemoveIndex (Variables|Default|GetLevelDeck))
    (Utilities|Array|Add (Variables|Default|GetCurrentDeck) _returnvalue_3)
    (Utilities|FlowControl|DoOnce false
      (:Completed
        (Variables|/Game/BP/Cards/BP_CardPar.BP_CardPar_C|SetIsActive _returnvalue_3 true))))
  (return))

(fn CreateLevelDeck
  (params (DeckData :type Map%20of%20Names%20to%20Integers))
  (bind _output_get (LocalVariables|SetDeckData%28local%29 DeckData))
  (bind _keys (Utilities|Map|Keys _output_get))
  (for _array_element _keys
    (for _index (range 1 (.Value (Utilities|Map|Find (LocalVariables|GetDeckData%28local%29) _array_element)))
      (Utilities|Array|Add (LocalVariables|GetLevelDeck%28local%29) _array_element)))
  (Variables|Default|SetLevelDeck (LocalVariables|GetLevelDeck%28local%29))
  (return))

(fn MoveCardRow
  (params (CardID :type BP%20Card%20Par%20Object%20Reference%20%28by%20ref%29))
  (if (Utilities|Array|ContainsItem (Variables|Default|GetRoadRow_01) CardID)
    (Utilities|Array|RemoveItem (Variables|Default|GetRoadRow_01) CardID)
    (for _array_element (Variables|Default|GetRoadRow_01)
      (Class|INTCard|MoveCard(Message) _array_element)
      (Utilities|FlowControl|DoOnce false
        (:Completed
          (Variables|/Game/BP/Cards/BP_CardPar.BP_CardPar_C|SetIsActive _array_element true))))
    (for _index (range 0 2)
      (Class|INTCard|VisibilityChange(Message) (Utilities|Array|Get(acopy) (Variables|Default|GetRoadRow_01) _index) true))
    (elif (Utilities|Array|ContainsItem (Variables|Default|GetRoadRow_02) CardID)
      (Utilities|Array|RemoveItem (Variables|Default|GetRoadRow_02) CardID)
      (for _array_element_2 (Variables|Default|GetRoadRow_02)
        (Class|INTCard|MoveCard(Message) _array_element_2)
        (Utilities|FlowControl|DoOnce false
          (:Completed
            (Variables|/Game/BP/Cards/BP_CardPar.BP_CardPar_C|SetIsActive _array_element_2 true))))
      (for _index_2 (range 0 2)
        (Class|INTCard|VisibilityChange(Message) (Utilities|Array|Get(acopy) (Variables|Default|GetRoadRow_02) _index_2) true))
      (elif (Utilities|Array|ContainsItem (Variables|Default|GetRoadRow_03) CardID)
        (Utilities|Array|RemoveItem (Variables|Default|GetRoadRow_03) CardID)
        (for _array_element_3 (Variables|Default|GetRoadRow_03)
          (Class|INTCard|MoveCard(Message) _array_element_3)
          (Utilities|FlowControl|DoOnce false
            (:Completed
              (Variables|/Game/BP/Cards/BP_CardPar.BP_CardPar_C|SetIsActive _array_element_3 true))))
        (for _index_3 (range 0 2)
          (Class|INTCard|VisibilityChange(Message) (Utilities|Array|Get(acopy) (Variables|Default|GetRoadRow_03) _index_3) true))
        (else
          (Development|PrintString "ERROR! Card ID not found in the RoadsRows! (bp_CardPlayerController: OpenCard)" true true "(R=1.000000,G=0.118750,B=0.000000,A=1.000000)" 4.0))))))

(fn SpawnCardsfromMainDeck
  (bind _output_get (LocalVariables|SetCardsInRow%28local%29 (/ (Utilities|Array|Length (Variables|Default|GetLevelDeck)) 3)))
  (for _index (range 0 (- _output_get 1))
    (bind _output_get_2 (Variables|Default|SetZoffset (+ (Variables|Default|GetZoffset) 3e+01)))
    (bind _output_get_3 (Variables|Default|SetStartingPosition (+ (Variables|Default|GetStartingPosition) (Variables|Default|GetYoffset))))
    (bind _returnvalue (Game|SpawnActorfromClass "/Game/BP/Cards/BP_CardPar.BP_CardPar_C" (Math|Transform|MakeTransform (Math|Vector|MakeVector 0.0 _output_get_3 _output_get_2) "0, 0, 0" "1.000000,1.000000,1.000000") "Undefined" "MultiplyWithRoot" 0 (Utilities|Array|Get(acopy) (Variables|Default|GetLevelDeck)) 0))
    (Utilities|Array|RemoveIndex (Variables|Default|GetLevelDeck))
    (Utilities|Array|Add (Variables|Default|GetRoadRow_01) _returnvalue)
    (Utilities|FlowControl|DoOnce false
      (:Completed
        (Variables|/Game/BP/Cards/BP_CardPar.BP_CardPar_C|SetIsActive _returnvalue true))))
  (Variables|Default|SetZoffset -3e+01)
  (Variables|Default|SetStartingPosition 2e+02)
  (for _index_2 (range 0 (- (LocalVariables|GetCardsInRow%28local%29) 1))
    (bind _output_get_4 (Variables|Default|SetZoffset (+ (Variables|Default|GetZoffset) 3e+01)))
    (bind _output_get_5 (Variables|Default|SetStartingPosition (+ (Variables|Default|GetStartingPosition) (Variables|Default|GetYoffset))))
    (bind _returnvalue_2 (Game|SpawnActorfromClass "/Game/BP/Cards/BP_CardPar.BP_CardPar_C" (Math|Transform|MakeTransform (Math|Vector|MakeVector 1.6e+02 _output_get_5 _output_get_4) "0, 0, 0" "1.000000,1.000000,1.000000") "Undefined" "MultiplyWithRoot" 0 (Utilities|Array|Get(acopy) (Variables|Default|GetLevelDeck)) 0))
    (Utilities|Array|RemoveIndex (Variables|Default|GetLevelDeck))
    (Utilities|Array|Add (Variables|Default|GetRoadRow_02) _returnvalue_2)
    (Utilities|FlowControl|DoOnce false
      (:Completed
        (Variables|/Game/BP/Cards/BP_CardPar.BP_CardPar_C|SetIsActive _returnvalue_2 true))))
  (Variables|Default|SetZoffset -3e+01)
  (Variables|Default|SetStartingPosition 2e+02)
  (for _index_3 (range 0 (- (LocalVariables|GetCardsInRow%28local%29) 1))
    (bind _output_get_6 (Variables|Default|SetZoffset (+ (Variables|Default|GetZoffset) 3e+01)))
    (bind _output_get_7 (Variables|Default|SetStartingPosition (+ (Variables|Default|GetStartingPosition) (Variables|Default|GetYoffset))))
    (bind _returnvalue_3 (Game|SpawnActorfromClass "/Game/BP/Cards/BP_CardPar.BP_CardPar_C" (Math|Transform|MakeTransform (Math|Vector|MakeVector 3.2e+02 _output_get_7 _output_get_6) "0, 0, 0" "1.000000,1.000000,1.000000") "Undefined" "MultiplyWithRoot" 0 (Utilities|Array|Get(acopy) (Variables|Default|GetLevelDeck)) 0))
    (Utilities|Array|RemoveIndex (Variables|Default|GetLevelDeck))
    (Utilities|Array|Add (Variables|Default|GetRoadRow_03) _returnvalue_3)
    (Utilities|FlowControl|DoOnce false
      (:Completed
        (Variables|/Game/BP/Cards/BP_CardPar.BP_CardPar_C|SetIsActive _returnvalue_3 true))))
  (Development|PrintString (Utilities|String|ToString(Integer) (Utilities|Array|Length (Variables|Default|GetLevelDeck))))
  (return))

(fn StartingCardsSetting
  (for _index (range 0 2)
    (Class|INTCard|VisibilityChange(Message) (Utilities|Array|Get(acopy) (Variables|Default|GetRoadRow_01) _index) true))
  (for _index_2 (range 0 2)
    (Class|INTCard|VisibilityChange(Message) (Utilities|Array|Get(acopy) (Variables|Default|GetRoadRow_02) _index_2) true))
  (for _index_3 (range 0 2)
    (Class|INTCard|VisibilityChange(Message) (Utilities|Array|Get(acopy) (Variables|Default|GetRoadRow_03) _index_3) true))
  (return))

(fn TrytoUseCard
  (params (CardID :type BP%20Card%20Par%20Object%20Reference))
  (CallFunction|MoveCardRow CardID)
  (return false))