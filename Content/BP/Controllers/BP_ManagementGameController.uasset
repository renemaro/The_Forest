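; BP_ManagementGameController is the controller for the management game, setting up its item data and UI on BeginPlay.
; It fetches an items map from the game instance, stores it as ItemsList and prints each key and value to screen as temporary debug output.
; It then creates the WG_ManagementUI widget with itself as owner, keeps a reference and adds it to the viewport.
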(event EventBeginPlay
  (Utilities|FlowControl|Sequence
    (:then_0
      (bind _itemslist (Class|INTGameInstance|GetItems(Message) (Game|GetGameInstance)))
      (bind _output_get (Variables|Default|SetItems%20List _itemslist))
      (bind _keys (Utilities|Map|Keys _output_get))
      (for _array_element _keys
        ;[1 0.9296 0.1244] TEMP
        (Development|PrintString (Utilities|String|Append (Utilities|String|ToString(Name) _array_element) " = " (Utilities|String|ToString(Integer) (.Value (Utilities|Map|Find (Variables|Default|GetItems%20List) _array_element)))))))
    (:then_1
      (bind _returnvalue (UserInterface|CreateWidget "/Game/UI/WG_ManagementUI.WG_ManagementUI_C" self))
      (bind _output_get_2 (Variables|Default|SetManagementUI _returnvalue))
      (UserInterface|Viewport|AddtoViewport _output_get_2 0))))

(fn ConstructionScript)